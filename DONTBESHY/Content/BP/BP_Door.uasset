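; Door Blueprint that teleports the top-down player character when it enters the trigger, hidden behind a screen fade.
; On overlap with BP_Char_topdown it shows a fade-on widget, waits briefly, then moves and rotates the character to the TpPos point.
; TpPos location is converted from actor-local to world space, while its rotation is applied as is.
; A fade-off widget then plays and is removed after a short delay.
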(event `self.Trigger.OnComponentBeginOverlap`
  (params (OverlappedComponent :type "PrimitiveComponent Object Reference") (OtherActor :type "Actor Object Reference") (OtherComp :type "PrimitiveComponent Object Reference") (OtherBodyIndex :type Integer) (bFromSweep :type Boolean) (SweepResult :type "HitResult Structure (by ref)"))
  (bind (_tp_pos_location _tp_pos_rotation) (`KismetMathLibrary.BreakTransform` (`self.Tp_pos`)))
  (bind _asbp_char_topdown (cast `/Game/Char/BP_Char_topdown` OtherActor)) ; ссылка на персонажа
  (bind _returnvalue (`|CreateWidget` "/Game/BP/WB_fade_on.WB_fade_on_C"))
  (`UserWidget.AddToViewport` _returnvalue 0)
  (`/Game/BP/WB_fade_on.Fade onn` _returnvalue)
  (`KismetSystemLibrary.Delay` 0.5)
  (`self.K2_SetActorLocationAndRotation` _asbp_char_topdown (`KismetMathLibrary.TransformLocation` (`self.GetTransform`) _tp_pos_location) _tp_pos_rotation false false)
  (`Widget.RemoveFromParent` _returnvalue)
  (bind _returnvalue_2 (`|CreateWidget` "/Game/BP/WB_fade_off.WB_fade_off_C"))
  (`UserWidget.AddToViewport` _returnvalue_2 0)
  (`/Game/BP/WB_fade_off.FadeOff` _returnvalue_2)
  (`KismetSystemLibrary.Delay` 0.5)
  (`Widget.RemoveFromParent` _returnvalue_2))

(fn `UserConstructionScript`)